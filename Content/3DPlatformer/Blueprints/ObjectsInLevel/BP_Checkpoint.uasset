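; Checkpoint actor for a 3D platformer that sets the player's respawn point when touched.
; Any overlap with its Box trigger removes the Widget component's widget from its parent.
; While unactivated, an overlap by BP_ThirdPersonCharacter writes the box location to that character's RespawnPosition, plays a fire sound and starts Niagara fire and poof effects.
; An IsActivated flag makes this activation one-time.
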(event `self.Box.OnComponentBeginOverlap`
  (params (OverlappedComponent :type "PrimitiveComponent Object Reference") (OtherActor :type "Actor Object Reference") (OtherComp :type "PrimitiveComponent Object Reference") (OtherBodyIndex :type Integer) (bFromSweep :type Boolean) (SweepResult :type "HitResult Structure (by ref)"))
  (`Widget.RemoveFromParent` (`WidgetComponent.GetWidget` (`self.Widget`)))
  (if (not (`self.IsActivated`))
    (bind _asbp_third_person_character (cast `/Game/ThirdPerson/Blueprints/BP_ThirdPersonCharacter` OtherActor))
    (set `/Game/ThirdPerson/Blueprints/BP_ThirdPersonCharacter.RespawnPosition` (`SceneComponent.K2_GetComponentLocation` (`self.Box`)) _asbp_third_person_character)
    (`GameplayStatics.PlaySound2D` "/Game/3DPlatformer/Assets/Sounds/FX/Fire_Cue.Fire_Cue" 1.0 1.0 0.0 null null)
    (`ActorComponent.Activate` (`self.Niagara_Fire`) false)
    (`ActorComponent.Activate` (`self.Niagara_Poof`) false)
    (set `self.IsActivated` true)))

(fn `UserConstructionScript`)