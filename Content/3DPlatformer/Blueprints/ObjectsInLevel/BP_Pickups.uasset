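; BP_Pickups is a level pickup for a 3D platformer that grants the player score, extra time or an extra life.
; A PickupList enum selects the reward, and the construction script swaps the static mesh to match that type.
; On overlap with BP_ThirdPersonCharacter it updates the character's Score, Timer or LifesNumber directly, then destroys itself.
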(event `self.ReceiveActorBeginOverlap`
  (params (OtherActor :type "Actor Object Reference"))
  (bind _asbp_third_person_character (cast `/Game/ThirdPerson/Blueprints/BP_ThirdPersonCharacter` OtherActor))
  (switch `/Game/3DPlatformer/Blueprints/ObjectsInLevel/E_Pickups` (`self.PickupList`)
    (:`NewEnumerator0`
      (set `/Game/ThirdPerson/Blueprints/BP_ThirdPersonCharacter.Score` (+ (`/Game/ThirdPerson/Blueprints/BP_ThirdPersonCharacter.Score` _asbp_third_person_character) (`self.ScoreEarned`)) _asbp_third_person_character))
    (:`NewEnumerator1`
      (set `/Game/ThirdPerson/Blueprints/BP_ThirdPersonCharacter.Timer` (+ (`/Game/ThirdPerson/Blueprints/BP_ThirdPersonCharacter.Timer` _asbp_third_person_character) (`self.TimerEarned`)) _asbp_third_person_character))
    (:`NewEnumerator2`
      (bind _result (`/Engine/EditorBlueprintResources/StandardMacros.IncrementInt` (`/Game/ThirdPerson/Blueprints/BP_ThirdPersonCharacter.LifesNumber` _asbp_third_person_character))
        (:`  `
          (set `/Game/ThirdPerson/Blueprints/BP_ThirdPersonCharacter.LifesNumber` _result _asbp_third_person_character)))))
  (`self.K2_DestroyActor`))

(fn `UserConstructionScript`
  (`StaticMeshComponent.SetStaticMesh` (`self.StaticMesh`) (select `/Game/3DPlatformer/Blueprints/ObjectsInLevel/E_Pickups` (`self.PickupList`) :`NewEnumerator0` "/Game/3DPlatformer/Assets/Objects/Apple/source/Apple.Apple" :`NewEnumerator1` "/Game/3DPlatformer/Assets/Objects/Timer/timer.timer" :`NewEnumerator2` "/Game/3DPlatformer/Assets/Objects/Panel/Panels/signs_sign1.signs_sign1" :!type "StaticMesh Object Reference")))