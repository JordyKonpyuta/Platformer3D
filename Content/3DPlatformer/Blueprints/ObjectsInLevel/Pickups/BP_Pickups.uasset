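; BP_Pickups is a collectible pickup for the 3D platformer that acts as an apple, timer or life, chosen by PickupList.
; The construction script picks the matching mesh, and a timeline started at BeginPlay animates it vertically by adding its value to the current Z.
; On overlap with BP_ThirdPersonCharacter, it increases that character's score, timer or life count, plays the matching sound and destroys itself.
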(event `self.ReceiveBeginPlay`
  (bind (_returnvalue_x _returnvalue_y _returnvalue_z) (`KismetMathLibrary.BreakVector` (`self.K2_GetActorLocation`)))
  (bind (_direction _animation) (`Timeline|Animation`)
    (:`Update`
      (`self.K2_SetActorLocation` (`KismetMathLibrary.MakeVector` _returnvalue_x _returnvalue_y (+ (.z _animation) _returnvalue_z))))))

(event `self.ReceiveActorBeginOverlap`
  (params (OtherActor :type "Actor Object Reference"))
  (bind _asbp_third_person_character (cast `/Game/ThirdPerson/Blueprints/BP_ThirdPersonCharacter` OtherActor))
  (switch `/Game/3DPlatformer/Blueprints/ObjectsInLevel/Pickups/E_Pickups` (`self.PickupList`)
    (:`NewEnumerator0`
      (set `/Game/ThirdPerson/Blueprints/BP_ThirdPersonCharacter.Score` (+ (`/Game/ThirdPerson/Blueprints/BP_ThirdPersonCharacter.Score` _asbp_third_person_character) (`self.ScoreEarned`)) _asbp_third_person_character)
      (`GameplayStatics.PlaySound2D` "/Game/3DPlatformer/Assets/Sounds/FX/Pickups/PickUpApple_Cue.PickUpApple_Cue" 1.0 1.0 0.0 null null))
    (:`NewEnumerator1`
      (set `/Game/ThirdPerson/Blueprints/BP_ThirdPersonCharacter.Timer` (+ (`/Game/ThirdPerson/Blueprints/BP_ThirdPersonCharacter.Timer` _asbp_third_person_character) (`self.TimerEarned`)) _asbp_third_person_character)
      (`GameplayStatics.PlaySound2D` "/Game/3DPlatformer/Assets/Sounds/FX/Pickups/PickUpTimer_Cue.PickUpTimer_Cue" 1.0 1.0 0.1 null null))
    (:`NewEnumerator2`
      (bind _result (`/Engine/EditorBlueprintResources/StandardMacros.IncrementInt` (`/Game/ThirdPerson/Blueprints/BP_ThirdPersonCharacter.LifesNumber` _asbp_third_person_character))
        (:`  `
          (set `/Game/ThirdPerson/Blueprints/BP_ThirdPersonCharacter.LifesNumber` _result _asbp_third_person_character)
          (`GameplayStatics.PlaySound2D` "/Game/3DPlatformer/Assets/Sounds/FX/Pickups/PickUpLife_Cue.PickUpLife_Cue" 1.0 1.0 0.1 null null)))))
  (`self.K2_DestroyActor`))

(fn `UserConstructionScript`
  (`StaticMeshComponent.SetStaticMesh` (`self.StaticMesh`) (select `/Game/3DPlatformer/Blueprints/ObjectsInLevel/Pickups/E_Pickups` (`self.PickupList`) :`NewEnumerator0` "/Game/3DPlatformer/Assets/Objects/Apple/source/Apple.Apple" :`NewEnumerator1` "/Game/3DPlatformer/Assets/Objects/Timer/timer.timer" :`NewEnumerator2` "/Game/3DPlatformer/Assets/Objects/genshin-destiny2-paimon-ghost/source/mni_donghua.mni_donghua" :!type "StaticMesh Object Reference")))