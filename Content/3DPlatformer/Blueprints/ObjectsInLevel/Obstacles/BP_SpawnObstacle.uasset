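; Level obstacle spawner that repeatedly spawns a barrel or trash bag at its own transform, rolled 90 degrees.
; BeginPlay runs an endless Delay loop, with a Select on an index choosing which class to spawn.
; When a trash bag begins overlapping its Box, it activates a Niagara effect and plays a 2D bag-destroyed sound, without destroying the bag itself.
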(event `self.ReceiveBeginPlay`
  (bind _returnvalue (`self.GetTransform`))
  (`KismetSystemLibrary.Delay` 5.5 :!label _label)
  (`|SpawnActorFromClass` (select `int` (`self.Index`) :`0` "/Game/3DPlatformer/Blueprints/ObjectsInLevel/Obstacles/BP_Barrel.BP_Barrel_C" :`1` "/Game/3DPlatformer/Blueprints/ObjectsInLevel/Obstacles/BP_TrashBag.BP_TrashBag_C" :!type "Actor Class Reference") (`KismetMathLibrary.MakeTransform` (.location _returnvalue) (`KismetMathLibrary.MakeRotator` (+ (.roll (.rotation _returnvalue)) 90.0) (.pitch (.rotation _returnvalue)) (.yaw (.rotation _returnvalue))) (.scale _returnvalue)) "Undefined" "MultiplyWithRoot" null null)
  (goto _label))

(event `self.Box.OnComponentBeginOverlap`
  (params (OverlappedComponent :type "PrimitiveComponent Object Reference") (OtherActor :type "Actor Object Reference") (OtherComp :type "PrimitiveComponent Object Reference") (OtherBodyIndex :type Integer) (bFromSweep :type Boolean) (SweepResult :type "HitResult Structure (by ref)"))
  (cast `/Game/3DPlatformer/Blueprints/ObjectsInLevel/Obstacles/BP_TrashBag` OtherActor)
  (`ActorComponent.Activate` (`self.Niagara`) false)
  (`GameplayStatics.PlaySound2D` "/Game/3DPlatformer/Assets/Sounds/FX/BagDestroyed_Cue.BagDestroyed_Cue" 1.0 1.0 0.0 null null))

(fn `UserConstructionScript`)