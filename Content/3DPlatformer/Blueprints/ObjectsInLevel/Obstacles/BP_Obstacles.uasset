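; BP_Obstacles is a placeable level obstacle for the 3D platformer that hurts the third-person character on contact.
; The construction script sets its static mesh from the ObstaclesList selection, either a banana peel or one of several cans.
; When its mesh hits a character that is neither dashing nor invincible, it calls TakeDamage on that character, plays a fall sound and destroys itself.
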(event `self.StaticMesh.OnComponentHit`
  (params (HitComponent :type "PrimitiveComponent Object Reference") (OtherActor :type "Actor Object Reference") (OtherComp :type "PrimitiveComponent Object Reference") (NormalImpulse :type "Vector Structure") (Hit :type "HitResult Structure (by ref)"))
  (bind _asbp_third_person_character (cast `/Game/ThirdPerson/Blueprints/BP_ThirdPersonCharacter` OtherActor))
  (if (and (not (`/Game/ThirdPerson/Blueprints/BP_ThirdPersonCharacter.IsDashing` _asbp_third_person_character)) (not (`/Game/ThirdPerson/Blueprints/BP_ThirdPersonCharacter.IsInvicible` _asbp_third_person_character)))
    (`/Game/ThirdPerson/Blueprints/BP_ThirdPersonCharacter.TakeDamage` _asbp_third_person_character)
    (`GameplayStatics.PlaySound2D` "/Game/3DPlatformer/Assets/Sounds/FX/UI/Fall_Cue.Fall_Cue" 1.0 1.0 0.1 null null)
    (`self.K2_DestroyActor`)))

(fn `UserConstructionScript`
  (`StaticMeshComponent.SetStaticMesh` (`self.StaticMesh`) (select `/Game/3DPlatformer/Blueprints/ObjectsInLevel/Obstacles/E_Obstacles` (`self.ObstaclesList`) :`NewEnumerator1` "/Game/3DPlatformer/Assets/Objects/Trashes/BananaPeel/banana_peel_banana.banana_peel_banana" :`NewEnumerator3` "/Game/3DPlatformer/Assets/Objects/Trashes/Cans/Cans_Can_01_GEO.Cans_Can_01_GEO" :`NewEnumerator4` "/Game/3DPlatformer/Assets/Objects/Trashes/Cans/Cans_Can_02_GEO.Cans_Can_02_GEO" :`NewEnumerator5` "/Game/3DPlatformer/Assets/Objects/Trashes/Cans/Cans_Can_03_GEO.Cans_Can_03_GEO" :!type "StaticMesh Object Reference")))