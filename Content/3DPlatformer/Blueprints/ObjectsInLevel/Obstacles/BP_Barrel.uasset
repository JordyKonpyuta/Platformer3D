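; BP_Barrel is a platformer obstacle that travels along a spline and damages the player on contact.
; On BeginPlay, the MoveBarrel timeline plays at a rate derived from TimeToComplete, moving and rotating the mesh by distance along the spline.
; A mesh hit on BP_ThirdPersonCharacter calls TakeDamage, plays a 2D hit sound and destroys the barrel.
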(event `self.ReceiveBeginPlay`
  (`self.MoveObject`))

(event `MoveObject`
  (bind _spline (`self.Spline`))
  (`TimelineComponent.SetPlayRate` (`self.MoveBarrel`) (/ 1.0 (`self.TimeToComplete`)))
  (bind (_direction _move) (`Timeline|MoveBarrel`)
    (:`Update`
      (bind _returnvalue (`KismetMathLibrary.Lerp` 0.0 (`SplineComponent.GetSplineLength` (`self.Spline`)) _move))
      (`SceneComponent.K2_SetWorldTransform` (`self.StaticMesh`) (`KismetMathLibrary.MakeTransform` (`SplineComponent.GetLocationAtDistanceAlongSpline` _spline _returnvalue "World") (`SplineComponent.GetRotationAtDistanceAlongSpline` _spline _returnvalue "Local")) false false))))

(event `self.StaticMesh.OnComponentHit`
  (params (HitComponent :type "PrimitiveComponent Object Reference") (OtherActor :type "Actor Object Reference") (OtherComp :type "PrimitiveComponent Object Reference") (NormalImpulse :type "Vector Structure") (Hit :type "HitResult Structure (by ref)"))
  (bind _asbp_third_person_character (cast `/Game/ThirdPerson/Blueprints/BP_ThirdPersonCharacter` OtherActor))
  (`/Game/ThirdPerson/Blueprints/BP_ThirdPersonCharacter.TakeDamage` _asbp_third_person_character)
  (`GameplayStatics.PlaySound2D` "/Game/3DPlatformer/Assets/Sounds/FX/UI/Hit_Cue.Hit_Cue" 1.0 1.0 0.0 null null)
  (`self.K2_DestroyActor`))

(fn `UserConstructionScript`)